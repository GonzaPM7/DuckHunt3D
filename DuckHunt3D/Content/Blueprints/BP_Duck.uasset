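; Duck target for a shooting game that spawns as a randomly chosen green, blue or red type with its own score.
; Tick animates it by swapping static meshes and moves it in the XZ plane, bouncing off limits while timers randomize direction.
; Die flashes the HUD, awards points and drops it with physics, flipping until it lands.
; It reports landing, or escape when CurrentGun is zero, to BP_DuckGameMode and destroys itself.
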(event `self.ReceiveBeginPlay`
  (`KismetSystemLibrary.PrintString` (`KismetTextLibrary.Conv_TextToString` (`|FormatText` "Speed {0}  IndChangeDirection {1}  Green  {2}% Blue {3}%" (`self.Speed`) (`self.IndTimeDirection`) (`self.%GreenDuck`) (`self.%BlueDuck`))))
  (`self.StartDuck`))

(event `self.ReceiveTick`
  (params (DeltaSeconds :type "Float (single-precision)"))
  (bind (_returnvalue_x _returnvalue_y) (`KismetMathLibrary.BreakVector` (`self.K2_GetActorLocation`)))
  (bind (_returnvalue_x_2 _returnvalue_y_2 _returnvalue_z) (`KismetMathLibrary.BreakVector` (`SceneComponent.K2_GetComponentLocation` (`self.Model`))))
  (bind (_returnvalue_x_3 _returnvalue_y_3 _returnvalue_z_2) (`KismetMathLibrary.BreakVector` (+ (* (`self.DeltaTime`) (`self.Speed`) (`KismetMathLibrary.Normal` (`self.CurrentDirection`))) (`self.K2_GetActorLocation`))))
  (if (== (`self.Dead`) false)
    (bind _output_get (set `self.DeltaTime` DeltaSeconds))
    (bind _output_get_2 (set `self.Timer` (+ _output_get (`self.Timer`))))
    (if (>= _output_get_2 (`self.FrameTime `))
      (`self.AnimationSystem`)
      (set `self.Timer` 0.0))
    (bind _asbp_duck_game_mode (cast `/Game/Blueprints/BP_DuckGameMode` (`GameplayStatics.GetGameMode`)))
    (if (== (`/Game/Blueprints/BP_DuckGameMode.CurrentGun` _asbp_duck_game_mode) 0)
      (`self.DuckEscapes`)
      (else
        (`self.CheckLimits`)
        (`self.K2_SetActorLocationAndRotation` (`KismetMathLibrary.MakeVector` _returnvalue_x_3 _returnvalue_y _returnvalue_z_2) (`KismetMathLibrary.MakeRotator` 0.0 0.0 (`self.Rotation`)))))
    (elif (<= _returnvalue_z 0.0)
      (`AudioComponent.Stop` (`self.DuckSound`))
      (`GameplayStatics.PlaySoundAtLocation` "/Game/Sounds/Drop.Drop" (`SceneComponent.K2_GetComponentLocation` (`self.Model`)) (struct) 1.0 1.0 0.0 null null null null)
      (bind _asbp_duck_game_mode_2 (cast `/Game/Blueprints/BP_DuckGameMode` (`GameplayStatics.GetGameMode`)))
      (`/Game/Blueprints/BP_DuckGameMode.NotifyDuckResult` _asbp_duck_game_mode_2 true)
      (`self.K2_DestroyActor`)
      (elif (`self.Fall`)
        (bind _output_get_3 (set `self.DeltaTime` DeltaSeconds))
        (bind _output_get_4 (set `self.Timer` (+ _output_get_3 (`self.Timer`))))
        (if (>= _output_get_4 (`self.FrameTime `))
          (set `self.Timer` 0.0)
          (if (== (`self.Rotation`) 0.0)
            (set `self.Rotation` 180.0)
            (else
              (set `self.Rotation` 0.0)))
          (`SceneComponent.K2_SetWorldRotation` (`self.Model`) (`KismetMathLibrary.MakeRotator` 0.0 0.0 (`self.Rotation`)) false false))))))

(event `AnimationDie`
  (bind _ducksound (`self.DuckSound`))
  (`KismetSystemLibrary.Delay` 0.5)
  (`StaticMeshComponent.SetStaticMesh` (`self.Model`) (`|GetArrayItem` (`self.FallDuck`) (select `/Game/Blueprints/E_TypeDucks` (`self.TypeDuck`) :`NewEnumerator1` 1 :`NewEnumerator2` 2)))
  (`PrimitiveComponent.SetSimulatePhysics` (`self.Model`) true)
  (`AudioComponent.SetSound` _ducksound "/Game/Sounds/Fall.Fall")
  (`AudioComponent.Play` _ducksound 0.0)
  (`|SpawnActorFromClass` "/Game/Blueprints/BP_DuckScore.BP_DuckScore_C" (`KismetMathLibrary.Conv_VectorToTransform` (`self.K2_GetActorLocation`)) "Undefined" "MultiplyWithRoot" null (select `/Game/Blueprints/E_TypeDucks` (`self.TypeDuck`) :`NewEnumerator0` "NewEnumerator0" :`NewEnumerator1` "NewEnumerator2" :`NewEnumerator2` "NewEnumerator1" :!type "/Game/Blueprints/E_DuckScore Enum") null)
  (bind _asbp_duck_game_mode (cast `/Game/Blueprints/BP_DuckGameMode` (`GameplayStatics.GetGameMode`)))
  (`/Game/Blueprints/BP_DuckGameMode.AddScore` _asbp_duck_game_mode (select `/Game/Blueprints/E_TypeDucks` (`self.TypeDuck`) :`NewEnumerator0` 500 :`NewEnumerator1` 1500 :`NewEnumerator2` 1000))
  (set `self.Fall` true))

(event `FlashCamera`
  (bind _asbp_duck_game_mode (cast `/Game/Blueprints/BP_DuckGameMode` (`GameplayStatics.GetGameMode`)))
  (bind _image_flash (`/Game/UI/WBP_HUD.Image_Flash` (`/Game/Blueprints/BP_DuckGameMode.HUD` _asbp_duck_game_mode)))
  (`Image.SetColorAndOpacity` _image_flash (struct :`R` 1.0 :`G` 1.0 :`B` 1.0 :`A` 0.5))
  (`KismetSystemLibrary.Delay` 0.1)
  (`Image.SetColorAndOpacity` _image_flash (struct :`R` 1.0 :`G` 1.0 :`B` 1.0)))

(fn `AnimationSystem`
  (if (== (select `/Game/Blueprints/E_TypeDucks` (`self.TypeDuck`) :`NewEnumerator0` 2 :`NewEnumerator1` 5 :`NewEnumerator2` 8) (`self.CurrentIndex `))
    (set `self.Index` -1.0)
    (elif (== (`self.CurrentIndex `) (select `/Game/Blueprints/E_TypeDucks` (`self.TypeDuck`) :`NewEnumerator1` 3 :`NewEnumerator2` 6))
      (set `self.Index` 1.0)))
  (set `self.CurrentIndex ` (`KismetMathLibrary.FTrunc` (+ (`self.CurrentIndex `) (`self.Index`))))
  (`StaticMeshComponent.SetStaticMesh` (`self.Model`) (`|GetArrayItem` (`self.CurrectDuckFrames`) (`self.CurrentIndex `)))
  (if (== (select `/Game/Blueprints/E_TypeDucks` (`self.TypeDuck`) :`NewEnumerator1` 3 :`NewEnumerator2` 6) (`self.CurrentIndex `))
    (`AudioComponent.Play` (`self.DuckSound`) 0.0)))

(fn `ChangeDirection`
  (set `self.CurrentDirection` (`KismetMathLibrary.MakeVector` (`KismetMathLibrary.RandomFloatInRange` -1.0 1.0) 0.0 (`KismetMathLibrary.RandomFloatInRange` -1.0 1.0)))
  (`self.ChangeFlyAnimation`)
  (`self.ProgramChangeDirection`))

(fn `ChangeFlyAnimation`
  (bind _currentdirection_x (`KismetMathLibrary.BreakVector` (`self.CurrentDirection`)))
  (if (>= (`KismetMathLibrary.RandomFloatInRange` -1.0 1.0) 0.0)
    (set `self.CurrectDuckFrames` (`self.DuckUp`))
    (else
      (set `self.CurrectDuckFrames` (`self.DuckHorizontal`))))
  (if (> _currentdirection_x 0.0)
    (set `self.Rotation` 0.0)
    (else
      (set `self.Rotation` 180.0))))

(fn `CheckLimits`
  (bind (_returnvalue_x _returnvalue_y _returnvalue_z) (`KismetMathLibrary.BreakVector` (`self.K2_GetActorLocation`)))
  (bind (_currentdirection_x _currentdirection_y _currentdirection_z) (`KismetMathLibrary.BreakVector` (`self.CurrentDirection`)))
  (bind (_currentdirection_x_2 _currentdirection_y_2 _currentdirection_z_2) (`KismetMathLibrary.BreakVector` (`self.CurrentDirection`)))
  (bind _returnvalue (`KismetMathLibrary.MakeVector` _currentdirection_x _currentdirection_y (* _currentdirection_z -1.0)))
  (bind _returnvalue_2 (`KismetMathLibrary.MakeVector` (* _currentdirection_x_2 -1.0) _currentdirection_y_2 _currentdirection_z_2))
  (if (> _returnvalue_x 1000.0)
    (set `self.CurrentDirection` _returnvalue_2)
    (`self.ChangeFlyAnimation` :!label _label)
    (elif (< _returnvalue_x -1000.0)
      (set `self.CurrentDirection` _returnvalue_2)
      (goto _label)
      (else
        _)))
  (if (> _returnvalue_z 800.0)
    (set `self.CurrentDirection` _returnvalue)
    (`self.ChangeFlyAnimation` :!label _label_2)
    (elif (< _returnvalue_z 0.0)
      (set `self.CurrentDirection` _returnvalue)
      (goto _label_2))))

(fn `Die`
  (set `self.Dead` true)
  (`self.FlashCamera`)
  (`StaticMeshComponent.SetStaticMesh` (`self.Model`) (`|GetArrayItem` (`self.DeadDuck`) (select `/Game/Blueprints/E_TypeDucks` (`self.TypeDuck`) :`NewEnumerator1` 1 :`NewEnumerator2` 2)))
  (`self.AnimationDie`))

(fn `DuckEscapes`
  (bind _asbp_duck_game_mode (cast `/Game/Blueprints/BP_DuckGameMode` (`GameplayStatics.GetGameMode`)))
  (`/Game/Blueprints/BP_DuckGameMode.NotifyDuckResult` _asbp_duck_game_mode false)
  (`self.K2_DestroyActor`))

(fn `ProgramChangeDirection`
  (bind _typeduck (`self.TypeDuck`))
  (`KismetSystemLibrary.K2_SetTimer` null "ChangeDirection" (`KismetMathLibrary.RandomFloatInRange` (* (select `/Game/Blueprints/E_TypeDucks` _typeduck :`NewEnumerator1` 2.0 :`NewEnumerator2` 4.0) (`self.IndTimeDirection`)) (* (select `/Game/Blueprints/E_TypeDucks` _typeduck :`NewEnumerator1` 4.0 :`NewEnumerator2` 6.0) (`self.IndTimeDirection`)))))

(fn `StartDuck`
  (bind _returnvalue (`KismetMathLibrary.RandomIntegerInRange` 0 100))
  (bind __greenduck (`self.%GreenDuck`))
  (bind _returnvalue_2 (+ (`self.%GreenDuck`) (`self.%BlueDuck`)))
  (if (and (>= _returnvalue 0) (< _returnvalue __greenduck))
    (set `self.TypeDuck` "NewEnumerator0" :!label _label)
    (set `self.CurrentIndex ` 0)
    (elif (and (>= _returnvalue __greenduck) (< _returnvalue _returnvalue_2))
      (set `self.TypeDuck` "NewEnumerator2")
      (set `self.CurrentIndex ` 6)
      (elif (and (>= _returnvalue _returnvalue_2) (< _returnvalue 100))
        (set `self.TypeDuck` "NewEnumerator1")
        (set `self.CurrentIndex ` 3)
        (else
          (goto _label)))))
  (set `self.CurrentDirection` (`KismetMathLibrary.MakeVector` (`KismetMathLibrary.RandomFloatInRange` -1.0 1.0) 0.0 (`KismetMathLibrary.RandomFloatInRange` 1.0 0.5)))
  (`self.ChangeFlyAnimation`)
  (`StaticMeshComponent.SetStaticMesh` (`self.Model`) (`|GetArrayItem` (`self.CurrectDuckFrames`) (`self.CurrentIndex `)))
  (`self.ProgramChangeDirection`))

(fn `UserConstructionScript`)