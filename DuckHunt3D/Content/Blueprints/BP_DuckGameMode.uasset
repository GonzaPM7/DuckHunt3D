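; Game mode for a duck shooting game that runs rounds and tracks score, ducks hit and shots.
; Each round spawns ducks one at a time through the first BP_DuckSpawner found, resetting the shot count per duck.
; NotifyDuckResult counts hits and spawns the next duck, ending the round at the quota.
; EndRound advances after a short delay if enough ducks were hit, otherwise restarts at round one with zero score.
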(event `self.ReceiveBeginPlay`
  (set `self.Score` 0)
  (`self.StartRound`))

(event `EndRound`
  (`KismetSystemLibrary.PrintString` (`KismetTextLibrary.Conv_TextToString` (`|FormatText` "Ronda: {0} Duck: {1}/{2}" (`self.CurrentRound`) (`self.DucksHit`) (`self.RequiredHits`))))
  (set `self.IsRoundActive` false)
  (if (>= (`self.DucksHit`) (`self.RequiredHits`))
    (`KismetSystemLibrary.Delay` 2.0)
    (bind _result (`/Engine/EditorBlueprintResources/StandardMacros.IncrementInt` (`self.CurrentRound`))
      (:`  `
        (set `self.CurrentRound` _result)))
    (else
      (set `self.Score` 0)
      (set `self.CurrentRound` 1)))
  (`self.StartRound`))

(fn `AddScore`
  (params (Score :type Integer))
  (set `self.Score` (+ Score (`self.Score`))))

(fn `NotifyDuckResult`
  (params (IsHit :type Boolean))
  (if IsHit
    (bind _result (`/Engine/EditorBlueprintResources/StandardMacros.IncrementInt` (`self.DucksHit`))
      (:`  `
        (set `self.DucksHit` _result))))
  (`self.SpawnNextDuck`))

(fn `SpawnNextDuck`
  (set `self.CurrentGun` (`self.MaxShotsPerDuck`))
  (`KismetSystemLibrary.PrintString` (`KismetTextLibrary.Conv_TextToString` (`|FormatText` "SpawnDuck Number{0} / {1}" (`self.DucksSpawned`) (`self.DucksPerRound`))))
  (if (< (`self.DucksSpawned`) (`self.DucksPerRound`))
    (bind _outactors (`GameplayStatics.GetAllActorsOfClass` "/Game/Blueprints/BP_DuckSpawner.BP_DuckSpawner_C"))
    (`/Game/Blueprints/BP_DuckSpawner.SpawnDuck` (`|GetArrayItem` _outactors))
    (bind _result (`/Engine/EditorBlueprintResources/StandardMacros.IncrementInt` (`self.DucksSpawned`))
      (:`  `
        (set `self.DucksSpawned` _result)))
    (else
      (`self.EndRound`))))

(fn `StartRound`
  (`KismetSystemLibrary.PrintString` "StartRound")
  (set `self.DucksSpawned` 0)
  (set `self.DucksHit` 0)
  (set `self.IsRoundActive` true)
  (`self.SpawnNextDuck`))

(fn `UserConstructionScript`)