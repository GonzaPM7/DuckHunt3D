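; BP_Train is a train actor that runs along a straight path and periodically restarts from where it was placed.
; BeginPlay saves the starting location and sets a timer for StartTrain, which moves the train back there and re-arms itself with a random 60–90 second delay.
; Tick shifts it along negative local X, adding delta time to the step rather than multiplying, so speed depends on frame rate.
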(event `self.ReceiveBeginPlay`
  (set `self.Location` (`self.K2_GetActorLocation`))
  (`KismetSystemLibrary.K2_SetTimer` null "StartTrain" (`KismetMathLibrary.RandomFloatInRange` 60.0 90.0)))

(event `self.ReceiveTick`
  (params (DeltaSeconds :type "Float (single-precision)"))
  (`self.K2_AddActorLocalOffset` (`KismetMathLibrary.MakeVector` (+ DeltaSeconds -5.0))))

(fn `StartTrain`
  (`self.K2_SetActorLocation` (`self.Location`))
  (`KismetSystemLibrary.K2_SetTimer` null "StartTrain" (`KismetMathLibrary.RandomFloatInRange` 60.0 90.0)))

(fn `UserConstructionScript`)